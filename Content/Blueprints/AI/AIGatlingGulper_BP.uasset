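; Gatling Gulper AI Blueprint that handles the enemy's dissolve effect on death.
; Each Tick, CheckIfDead copies the IsDead flag into DissolveMaterial.
; While that is true, Tick calls CreateDynamicMaterialInstance on mesh element 0 and plays a timeline that drives its "Amount" scalar parameter.
; The material call and timeline Play repeat every frame while dead, and nothing in these graphs sets IsDead.
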(event `self.ReceiveTick`
  (params (DeltaSeconds :type "Float (single-precision)"))
  (`self.CheckIfDead`)
  (if (`self.DissolveMaterial`)
    (bind _returnvalue (`PrimitiveComponent.CreateDynamicMaterialInstance` (`self.Mesh`) 0 null "None"))
    (bind (_direction _newtrack_1) (`Timeline|Timeline_0`)
      (:`Update`
        (`MaterialInstanceDynamic.SetScalarParameterValue` _returnvalue "Amount" _newtrack_1)))))

(fn `CheckIfDead`
  (if (`self.bIsDead`)
    (set `self.DissolveMaterial` true)
    (else
      (set `self.DissolveMaterial` false)))
  (return))

(fn `UserConstructionScript`)