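; Base Blueprint for the Queen Squid AI, handling its laser visual and death dissolve.
; Every Tick spawns a new attached beam emitter at LaserBegin, ending at a Visibility trace hit along LaserArrowPointer or at maximum range.
; Tick also copies IsDead to DissolveMaterial through CheckIfDead.
; While set, it recreates dynamic instances for four mesh material slots each frame and plays a timeline driving their Amount parameter.
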(event `self.ReceiveTick`
  (params (DeltaSeconds :type "Float (single-precision)"))
  (bind _mesh (`self.Mesh`))
  (bind _returnvalue (`SceneComponent.K2_GetComponentLocation` (`self.LaserBegin`)))
  (`|ExecutionSequence`
    (:`then_0`
      (bind _returnvalue_2 (`GameplayStatics.SpawnEmitterAttached` "/Game/HookGameAssets/Enemy/Queen_SquidBird/Particles/SquidQueenLaser.SquidQueenLaser" (`self.LaserBegin`)))
      (`ParticleSystemComponent.SetBeamSourcePoint` _returnvalue_2 0 _returnvalue 0)
      (bind _outhit (`KismetSystemLibrary.LineTraceSingle` _returnvalue (+ _returnvalue (* (`SceneComponent.GetForwardVector` (`self.Laser Arrow Pointer`)) 2000.0)) "TraceTypeQuery1"))
      (bind (_bblockinghit _binitialoverlap _time _distance _location _impactpoint _normal _impactnormal _physmat _hitactor _hitcomponent _hitbonename _hititem _faceindex _tracestart _traceend) (`GameplayStatics.BreakHitResult` _outhit))
      (`ParticleSystemComponent.SetBeamTargetPoint` _returnvalue_2 0 (`KismetMathLibrary.SelectVector` _location _traceend _bblockinghit) 0))
    (:`then_1`
      (`self.CheckIfDead`)
      (if (`self.Dissolve Material`)
        (`|ExecutionSequence`
          (:`then_0`
            (bind _returnvalue_3 (`PrimitiveComponent.CreateDynamicMaterialInstance` _mesh 1 null "None"))
            (bind (_direction _newtrack_1) (`Timeline|Timeline_0` :!label _label)
              (:`Update`
                (`MaterialInstanceDynamic.SetScalarParameterValue` (stale _returnvalue_4) "Amount" _newtrack_1)
                (`MaterialInstanceDynamic.SetScalarParameterValue` _returnvalue_3 "Amount" _newtrack_1)
                (`MaterialInstanceDynamic.SetScalarParameterValue` (stale _returnvalue_5) "Amount" _newtrack_1)
                (`MaterialInstanceDynamic.SetScalarParameterValue` (stale _returnvalue_6) "Amount" _newtrack_1))))
          (:`then_1`
            (bind _returnvalue_4 (`PrimitiveComponent.CreateDynamicMaterialInstance` _mesh 0 null "None"))
            (goto _label))
          (:`then_2`
            (bind _returnvalue_5 (`PrimitiveComponent.CreateDynamicMaterialInstance` _mesh 2 null "None"))
            (goto _label))
          (:`then_3`
            (bind _returnvalue_6 (`PrimitiveComponent.CreateDynamicMaterialInstance` _mesh 3 null "None"))
            (goto _label)))))))

(fn `CheckIfDead`
  (if (`self.bIsDead`)
    (set `self.Dissolve Material` true)
    (else
      (set `self.Dissolve Material` false)))
  (return))

(fn `UserConstructionScript`)