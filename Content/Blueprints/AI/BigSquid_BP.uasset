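; BigSquid is an AI squid Blueprint that plays a material dissolve effect when it dies.
; Tick calls CheckIfDead, which copies IsDead into DissolveMaterial.
; While that flag is set, every tick calls CreateDynamicMaterialInstance on three mesh slots and plays a timeline driving their "Amount" parameter.
; StartDissolve is an empty stub that only checks the flag.
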(event `self.ReceiveTick`
  (params (DeltaSeconds :type "Float (single-precision)"))
  (bind _mesh (`self.Mesh`))
  (`self.CheckIfDead`)
  (if (`self.bDissolveMaterial`)
    (`|ExecutionSequence`
      (:`then_0`
        (bind _returnvalue (`PrimitiveComponent.CreateDynamicMaterialInstance` _mesh 1 null "None"))
        (bind (_direction _newtrack_1) (`Timeline|Timeline_0` :!label _label)
          (:`Update`
            (`MaterialInstanceDynamic.SetScalarParameterValue` (stale _returnvalue_2) "Amount" _newtrack_1)
            (`MaterialInstanceDynamic.SetScalarParameterValue` _returnvalue "Amount" _newtrack_1)
            (`MaterialInstanceDynamic.SetScalarParameterValue` (stale _returnvalue_3) "Amount" _newtrack_1))))
      (:`then_1`
        (bind _returnvalue_2 (`PrimitiveComponent.CreateDynamicMaterialInstance` _mesh 0 null "None"))
        (goto _label))
      (:`then_2`
        (bind _returnvalue_3 (`PrimitiveComponent.CreateDynamicMaterialInstance` _mesh 2 null "None"))
        (goto _label)))))

(fn `CheckIfDead`
  (if (`self.bIsDead`)
    (set `self.bDissolveMaterial` true)
    (else
      (set `self.bDissolveMaterial` false)))
  (return))

(fn `StartDissolve`
  (if (`self.bDissolveMaterial`)
    (return)))

(fn `UserConstructionScript`)