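; Base player character Blueprint that handles pausing the game through a pause menu widget.
; The Pause input calls PauseGame, which pauses, lazily creates and shows the menu, switches to Game and UI input with a visible cursor, and sets InMenu.
; UnpauseGame resumes play, removes the menu and clears InMenu, without restoring input mode or cursor.
; InteractCheck is an empty stub, and a questions UI toggle sits unconnected.
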(event `InputAction|Pause`
  (params (Key :type "Key Structure"))
  ;[1 1 1] Pause the game
  (:`Pressed`
    (`self.PauseGame`)))

(fn `InteractCheck`)

(fn `PauseGame`
  (`GameplayStatics.SetGamePaused` true)
  (`/Engine/EditorBlueprintResources/StandardMacros.IsValid` (`self.Pause Menu`)
    (:`Is Valid`
      _)
    (:`Is Not Valid`
      (bind _returnvalue (`|CreateWidget` "/Game/UI/PauseMenu.PauseMenu_C" (`GameplayStatics.GetPlayerController` 0)))
      (set `self.Pause Menu` _returnvalue)))
  (`UserWidget.AddToViewport` (`self.Pause Menu`) 0)
  (`WidgetBlueprintLibrary.SetInputMode_GameAndUIEx` (`GameplayStatics.GetPlayerController` 0) (`self.Pause Menu`))
  (set `PlayerController.bShowMouseCursor` true (`GameplayStatics.GetPlayerController` 0))
  (set `self.bInMenu` true))

(fn `UnpauseGame`
  (`GameplayStatics.SetGamePaused` false)
  (`Widget.RemoveFromParent` (`self.Pause Menu`))
  (set `self.bInMenu` false))

(fn `UserConstructionScript`)